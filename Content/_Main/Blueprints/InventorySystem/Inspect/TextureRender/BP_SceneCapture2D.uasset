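; Scene capture helper in the inventory system's inspect feature that renders to the TextureInspect2D target.
; On BeginPlay it spawns a separate SceneCapture2D at its own transform, owned by the player pawn, and stores it as Render.
; The Settexture event assigns the target to that capture's component and prints the capture's name for debugging.
; Unconnected SetActive nodes for toggling capture never run.
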(event `self.ReceiveBeginPlay`
  (bind _returnvalue (`|SpawnActorFromClass` "/Script/Engine.SceneCapture2D" (`self.GetTransform`) "Undefined" "MultiplyWithRoot" (`GameplayStatics.GetPlayerPawn` 0) null))
  (set `self.Render` _returnvalue))

(event `Set texture`
  (bind _render (`self.Render`))
  (set `SceneCaptureComponent2D.TextureTarget` "/Game/_Main/Blueprints/InventorySystem/Inspect/TextureRender/TextureInspect2D.TextureInspect2D" (`SceneCapture2D.CaptureComponent2D` _render))
  (`KismetSystemLibrary.PrintString` (`KismetSystemLibrary.GetDisplayName` _render) true true (struct :`G` 0.66 :`B` 1.0 :`A` 1.0) 15.0))

(fn `UserConstructionScript`)