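; Inventory component holding five item slots, with camera line-trace interaction through ITF_Interact.
; AdicionarItem recursively fills matching stacks and empty slots up to each class's maximum, returning any remainder; slot changes refresh the local menu grid.
; UsarItem calls use on an existing or spawned item actor, removing consumables.
; LargarItem empties a slot, spawns its pickup ahead of the camera via Server events, and resets a matching player state.
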(event `self.ReceiveBeginPlay`
  (`KismetArrayLibrary.Array_Resize` (`self.InventorySlots`) 5))

(event `Att`
  (params (Index :type Integer))
  (`self.Atualizar a widget do inventario` Index))

(event `Disparar Traço de linha`
  (params (CharacterRef :type "/Game/_Main/Blueprints/Player/BP_CharMAIN Object Reference"))
  (bind _success_ (`self.Traço de linha para interagir`))
  (if _success_
    (`self.Interagir` CharacterRef)))

(event `Server Spawn Actor`
  (params (Class :type "Actor Class Reference") (Start :type "Vector Structure") (End :type "Vector Structure"))
  (bind _outhit (`KismetSystemLibrary.LineTraceSingle` :`Start` Start :`End` End :`TraceChannel` "TraceTypeQuery1" :`DrawDebugType` "Persistent"))
  (bind (_bblockinghit _binitialoverlap _time _distance _location _impactpoint _normal _impactnormal _physmat _hitactor _hitcomponent _hitbonename _bonename _hititem _elementindex _faceindex _tracestart _traceend) (`GameplayStatics.BreakHitResult` _outhit))
  (bind _returnvalue (`|SpawnActorFromClass` Class (`KismetMathLibrary.MakeTransform` (`KismetMathLibrary.SelectVector` _location _traceend)) "Undefined" "MultiplyWithRoot" null null))
  (message `/Game/Inventory/Interfaces/ITF_SetarQuantidadeDeItem.Setar Nova Quantidade` _returnvalue (`self.LargarItemAmount`)))

(event `Server Set Amount`
  (params (LargarItemAmount :type Integer))
  (set `self.LargarItemAmount` LargarItemAmount))

(event `ServerSpawn`
  (params (Class :type "Actor Class Reference") (`Spawn Transform Location` :type "Vector Structure") (`Spawn Transform Rotation` :type "Rotator Structure") (`Spawn Transform Scale` :type "Vector Structure"))
  (`self.MulticastSpawn` Class `Spawn Transform Location` `Spawn Transform Rotation` `Spawn Transform Scale`))

(event `MulticastSpawn`
  (params (Class :type "Actor Class Reference") (`Spawn Transform Location` :type "Vector Structure") (`Spawn Transform Rotation` :type "Rotator Structure") (`Spawn Transform Scale` :type "Vector Structure"))
  (`|SpawnActorFromClass` Class (`KismetMathLibrary.MakeTransform` `Spawn Transform Location` `Spawn Transform Rotation` `Spawn Transform Scale`) "Undefined" "MultiplyWithRoot" null null))

(fn `Adicionar Item`
  (params (Item :type "/Game/_Main/Blueprints/InventorySystem/ActosInventory/BP_InventoryDefault Class Reference") (Quantidade :type Integer))
  (returns (`Success?` :type Boolean) (Remainder :type Integer))
  (locals (`Local Item` :type "/Game/_Main/Blueprints/InventorySystem/ActosInventory/BP_InventoryDefault Class Reference") (`Local Quantidade de item` :type Integer) (`Local Quantidade Maxima de Items` :type Integer) (`Local index` :type Integer :default 0))
  (bind (_success_ _index) (`self.Verificar um slot vazio`))
  (bind (_success__2 _index_2) (`self.Verificar um slot vazio`))
  (bind _local_index (`local.Local index`))
  (bind (_item_struct_nomedoitem _item_struct_icone _item_struct_quantidademaximadeitems) (break `/Game/Inventory/Structs/S_ItemData` (defaults `Object` (`local.Local Item`))))
  (bind _returnvalue (- (`local.Local Quantidade de item`) 1))
  (bind _returnvalue_2 (+ (`.Amount` (`self.Obter dados do item no indice` (`local.Local index`))) (`local.Local Quantidade de item`)))
  (set `local.Local Item` Item)
  (set `local.Local Quantidade de item` Quantidade)
  (set `local.Local Quantidade Maxima de Items` _item_struct_quantidademaximadeitems)
  (if (> _item_struct_quantidademaximadeitems 1)
    (bind (_success__3 _index_3) (`self.Verificar Slot Livre` (`local.Local Item`)))
    (if _success__3
      (set `local.Local index` _index_3)
      (if (> _returnvalue_2 (`local.Local Quantidade Maxima de Items`))
        (set `local.Local Quantidade de item` (- _returnvalue_2 (`local.Local Quantidade Maxima de Items`)))
        (`KismetArrayLibrary.Array_Set` (`self.InventorySlots`) (`local.Local index`) (make `/Game/Inventory/Structs/S_InventoryItems` (`local.Local Item`) (`local.Local Quantidade Maxima de Items`)))
        (`self.Atualizar a widget do inventario` (`local.Local index`))
        (bind (_success__4 _remainder) (`self.Adicionar Item` (`local.Local Item`) (`local.Local Quantidade de item`)))
        (return true _remainder)
        (else
          (`KismetArrayLibrary.Array_Set` (`self.InventorySlots`) (`local.Local index`) (make `/Game/Inventory/Structs/S_InventoryItems` (`local.Local Item`) _returnvalue_2))
          (`self.Atualizar a widget do inventario` (`local.Local index`))
          (return true 0)))
      (elif _success_
        (set `local.Local index` _index)
        (if (> (`local.Local Quantidade de item`) (`local.Local Quantidade Maxima de Items`))
          (`KismetArrayLibrary.Array_Set` (`self.InventorySlots`) (`local.Local index`) (make `/Game/Inventory/Structs/S_InventoryItems` (`local.Local Item`) (`local.Local Quantidade Maxima de Items`)))
          (`self.Atualizar a widget do inventario` _local_index)
          (bind (_success__5 _remainder_2) (`self.Adicionar Item` (`local.Local Item`) (- (`local.Local Quantidade de item`) (`local.Local Quantidade Maxima de Items`))))
          (return true _remainder_2)
          (else
            (`/Engine/EditorBlueprintResources/StandardMacros.DoOnce` false
              (:`Completed`
                (`KismetArrayLibrary.Array_Set` (`self.InventorySlots`) (`local.Local index`) (make `/Game/Inventory/Structs/S_InventoryItems` (`local.Local Item`) (`local.Local Quantidade de item`)))
                (`self.Atualizar a widget do inventario` _local_index)
                (return true 0)))))
        (else
          (return false (`local.Local Quantidade de item`)))))
    (elif _success__2
      (set `local.Local index` _index_2)
      (`KismetArrayLibrary.Array_Set` (`self.InventorySlots`) (`local.Local index`) (make `/Game/Inventory/Structs/S_InventoryItems` (`local.Local Item`) 1))
      (`self.Atualizar a widget do inventario` (`local.Local index`))
      (if (> _returnvalue 0)
        (bind (_success__6 _remainder_3) (`self.Adicionar Item` (`local.Local Item`) _returnvalue))
        (return true _remainder_3)
        (else
          (return true 0)))
      (else
        (`KismetSystemLibrary.PrintString` "Não a slots disponiveis :/" true true (struct :`R` 1.0 :`G` 0.069327 :`A` 1.0) 5.0)
        (return false (`local.Local Quantidade de item`))))))

(fn `Atualizar a widget do inventario`
  (params (Index :type Integer))
  (if (`Controller.IsLocalController` (`GameplayStatics.GetPlayerController` 0))
    (`KismetSystemLibrary.PrintString` (`KismetStringLibrary.Conv_IntToString` Index))
    (`/Game/Inventory/W_InventorySlot.Atualizar Slots` (`|GetArrayItem` (`/Game/Inventory/W_InventoryGrid.SlotsArrayInventory` (`/Game/Wtestes/W_MainMenu.W_InventoryGrid` (`/Game/_Main/Blueprints/Player/BP_CharMAIN_Controller.Main Menu` (cast `/Game/_Main/Blueprints/Player/BP_CharMAIN_Controller` (`GameplayStatics.GetPlayerController` 0) :!pure true)))) Index))))

(fn `Interagir`
  (params (Character :type "/Game/_Main/Blueprints/Player/BP_CharMAIN Object Reference"))
  (bind (_bblockinghit _binitialoverlap _time _distance _location _impactpoint _normal _impactnormal _physmat _hitactor) (`GameplayStatics.BreakHitResult` (`self.Hit`)))
  (if (`KismetSystemLibrary.DoesImplementInterface` _hitactor "/Game/Inventory/Interfaces/ITF_Interact.ITF_Interact_C")
    (message `/Game/Inventory/Interfaces/ITF_Interact.Interact` _hitactor Character)))

(fn `Largar item`
  (params (Index :type Integer))
  (locals (`Local Index` :type Integer) (`Local Amount` :type Integer :default 0) (`Local Item` :type "/Game/_Main/Blueprints/InventorySystem/ActosInventory/BP_InventoryDefault Class Reference"))
  (bind _returnvalue (`GameplayStatics.GetPlayerPawn` 0))
  (bind _returnvalue_2 (`GameplayStatics.GetPlayerCameraManager` 0))
  (bind _local_index (`local.Local Index`))
  (bind (_item_struct_nomedoitem _item_struct_icone _item_struct_quantidademaximadeitems _item_struct_usavel_ _item_struct_consumivel_ _item_struct_dropavel_ _item_struct_pgv_ _item_struct_descricao _item_struct_estadodojogador) (break `/Game/Inventory/Structs/S_ItemData` (defaults `Object` (`local.Local Item`))))
  (bind _returnvalue_3 (`SceneComponent.K2_GetComponentLocation` (`PlayerCameraManager.TransformComponent` _returnvalue_2)))
  (bind _output_get (set `local.Local Index` Index))
  (bind (_item _amount) (`self.Obter dados do item no indice` _output_get))
  (set `local.Local Item` _item)
  (set `local.Local Amount` _amount)
  (`self.Server Set Amount` _amount)
  (if (> (`local.Local Amount`) 0)
    (for _ (range (`local.Local Amount`))
      (`self.Remover item` _local_index))
    (`self.Atualizar a widget do inventario` _local_index)
    (`self.Server Spawn Actor` (`.PGV?_20_5CAAFDCE4FC455A963F475A8DEB0061A` (break `/Game/Inventory/Structs/S_ItemData` (defaults `Object` (`local.Local Item`)))) _returnvalue_3 (+ _returnvalue_3 (* (`Actor.GetActorForwardVector` _returnvalue_2) 200.0)))
    (bind _playerstate (message `/Game/_Main/Blueprints/Player/States/Interfaces/ITF_EstadoDoJogador.Get Player State` _returnvalue))
    (bind _returnvalue_4 (`|EnumEquality` _playerstate _item_struct_estadodojogador))
    (if _returnvalue_4
      (message `/Game/_Main/Blueprints/Player/States/Interfaces/ITF_EstadoDoJogador.Set PlayerState` _returnvalue "NewEnumerator0")
      (`KismetSystemLibrary.PrintString` (`KismetStringLibrary.Conv_BoolToString` _returnvalue_4)))))

(fn `Obter dados do item no indice`
  (params (Index :type Integer))
  (returns (Item :type "/Game/_Main/Blueprints/InventorySystem/ActosInventory/BP_InventoryDefault Class Reference") (Amount :type Integer))
  (bind (_item _amount) (break `/Game/Inventory/Structs/S_InventoryItems` (`|GetArrayItem` (`self.InventorySlots`) Index)))
  (return _item _amount))

(fn `Remover item`
  (params (Index :type Integer))
  (bind (_item _amount) (`self.Obter dados do item no indice` Index))
  (if (> _amount 1)
    (`KismetArrayLibrary.Array_Set` (`self.InventorySlots`) Index (make `/Game/Inventory/Structs/S_InventoryItems` _item (- _amount 1)))
    (else
      (`KismetArrayLibrary.Array_Set` (`self.InventorySlots`) Index (make `/Game/Inventory/Structs/S_InventoryItems` null))))
  (`self.Atualizar a widget do inventario` (`local.Index`)))

(fn `Traço de linha para interagir`
  (returns (`Success?` :type Boolean))
  (bind _returnvalue (`GameplayStatics.GetPlayerCameraManager` 0))
  (bind _returnvalue_2 (`Actor.K2_GetActorLocation` _returnvalue))
  (bind (_outhit _returnvalue_3) (`KismetSystemLibrary.LineTraceSingle` _returnvalue_2 (+ _returnvalue_2 (* (`KismetMathLibrary.GetForwardVector` (`SceneComponent.K2_GetComponentRotation` (`Actor.RootComponent` _returnvalue))) 500.0)) "TraceTypeQuery1"))
  (if _returnvalue_3
    (set `self.Hit` _outhit)
    (return true)
    (else
      (return false))))

(fn `Usar Item`
  (params (index :type Integer))
  (locals (`Local Index` :type Integer))
  (bind _output_get (set `local.Local Index` index))
  (bind (_item _amount) (`self.Obter dados do item no indice` _output_get))
  (if (> _amount 0)
    (bind _returnvalue (`GameplayStatics.GetActorOfClass` _item))
    (`/Engine/EditorBlueprintResources/StandardMacros.IsValid` _returnvalue
      (:`Is Valid`
        (`/Game/_Main/Blueprints/InventorySystem/ActosInventory/BP_InventoryDefault.Usar Item` _returnvalue))
      (:`Is Not Valid`
        (bind _returnvalue_2 (`|SpawnActorFromClass` _item (`KismetMathLibrary.MakeTransform` (0.0 0.0 0.0)) "Undefined" "MultiplyWithRoot" null null))
        (`/Game/_Main/Blueprints/InventorySystem/ActosInventory/BP_InventoryDefault.Usar Item` _returnvalue_2)))
    (bind (_item_struct_nomedoitem _item_struct_icone _item_struct_quantidademaximadeitems _item_struct_usavel_ _item_struct_consumivel_) (break `/Game/Inventory/Structs/S_ItemData` (defaults `Object` _item)))
    (if _item_struct_consumivel_
      (`self.Remover item` (`local.Local Index`)))))

(fn `Verificar Slot Livre`
  (params (Item :type "/Game/_Main/Blueprints/InventorySystem/ActosInventory/BP_InventoryDefault Class Reference"))
  (returns (`Success?` :type Boolean) (Index :type Integer))
  (locals (lsuccess :type Boolean) (localindex :type Integer))
  (bind (_item_struct_nomedoitem _item_struct_icone _item_struct_quantidademaximadeitems) (break `/Game/Inventory/Structs/S_ItemData` (defaults `Object` Item)))
  (for (_array_element _array_index) (`self.InventorySlots`)
    (bind (_item _amount) (break `/Game/Inventory/Structs/S_InventoryItems` _array_element))
    (if (and (== _item Item) (< _amount _item_struct_quantidademaximadeitems))
      (set `local.lsuccess` true)
      (set `local.localindex` _array_index)
      (break)
      (else
        (set `local.lsuccess` false))))
  (return (`local.lsuccess`) (`local.localindex`)))

(fn `Verificar um slot vazio`
  (returns (`Success?` :type Boolean) (Index :type Integer))
  (locals (localsuccess :type Boolean) (localindex :type Integer))
  (for (_array_element _array_index) (`self.InventorySlots`)
    (if (`KismetSystemLibrary.IsValidClass` (`.Item_3_936F082242D12CED24DEC89682334765` (break `/Game/Inventory/Structs/S_InventoryItems` _array_element)))
      (set `local.localsuccess` false)
      (else
        (set `local.localsuccess` true)
        (set `local.localindex` _array_index)
        (break))))
  (return (`local.localsuccess`) (`local.localindex`)))